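; BP_Gun is a grabbable VR gun that fires a projectile from its muzzle.
; When its grab component reports a grab, it enables player input and adds the weapon mapping context for the grabbing hand, removing both on drop.
; The shoot action matching that hand spawns the projectile at the muzzle transform, with the player pawn as instigator.
; Left fire responds to Triggered, while right fire responds to Started.
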(event OnGrabbed(BP_GrabComponent)
  (Input|EnableInput (Game|GetPlayerController 0))
  (Input|AddMappingContext (PlayerController|LocalPlayerSubsystems|GetEnhancedInputLocalPlayerSubsystem (Game|GetPlayerController 0)) (select (Utilities|Enum|Equal(Enum) (Default|GetGrabbingHandType (Variables|Default|GetBP_GrabComponent)) "Left") "/Game/Input/IMC_VR_WeaponLeft.IMC_VR_WeaponLeft" "/Game/Input/IMC_VR_WeaponRight.IMC_VR_WeaponRight") 0 "(bIgnoreAllPressedKeysUntilRelease=True,bForceImmediately=False)"))

(event OnDropped(BP_GrabComponent)
  (Input|DisableInput (Game|GetPlayerController 0))
  (Input|RemoveMappingContext (PlayerController|LocalPlayerSubsystems|GetEnhancedInputLocalPlayerSubsystem (Game|GetPlayerController 0)) (select (Utilities|Enum|Equal(Enum) (Default|GetGrabbingHandType (Variables|Default|GetBP_GrabComponent)) "Left") "/Game/Input/IMC_VR_WeaponLeft.IMC_VR_WeaponLeft" "/Game/Input/IMC_VR_WeaponRight.IMC_VR_WeaponRight") "(bIgnoreAllPressedKeysUntilRelease=True,bForceImmediately=False)"))

(event Input|EnhancedActionEvents|EnhancedInputActionIA_VR_ShootLeft
  (params (ActionValue :type Float%20%28double-precision%29) (ElapsedSeconds :type Float%20%28double-precision%29) (TriggeredSeconds :type Float%20%28double-precision%29) (InputAction :type Input%20Action%20Object%20Reference :default "/Game/Input/Actions/IA_VR_ShootLeft.IA_VR_ShootLeft"))
  (bind _muzzlelocation (Variables|Default|GetMuzzleLocation))
  (:Triggered
    (if (Utilities|Enum|Equal(Enum) (Default|GetGrabbingHandType (Variables|Default|GetBP_GrabComponent)) "Left")
      (Game|SpawnActorfromClass "/Game/Sample/VRTemplate/Blueprints/Projectile.Projectile_C" (Math|Transform|MakeTransform (Transformation|GetWorldLocation _muzzlelocation) (Transformation|GetWorldRotation _muzzlelocation)) "AlwaysSpawn" self (Game|Player|GetPlayerPawn 0)))))

(event Input|EnhancedActionEvents|EnhancedInputActionIA_VR_ShootRight
  (params (ActionValue :type Float%20%28double-precision%29) (ElapsedSeconds :type Float%20%28double-precision%29) (TriggeredSeconds :type Float%20%28double-precision%29) (InputAction :type Input%20Action%20Object%20Reference :default "/Game/Input/Actions/IA_VR_ShootRight.IA_VR_ShootRight"))
  (bind _muzzlelocation (Variables|Default|GetMuzzleLocation))
  (:Started
    (if (Utilities|Enum|Equal(Enum) (Default|GetGrabbingHandType (Variables|Default|GetBP_GrabComponent)) "Right")
      (Game|SpawnActorfromClass "/Game/Sample/VRTemplate/Blueprints/Projectile.Projectile_C" (Math|Transform|MakeTransform (Transformation|GetWorldLocation _muzzlelocation) (Transformation|GetWorldRotation _muzzlelocation)) "AlwaysSpawn" self (Game|Player|GetPlayerPawn 0)))))

(event EventBeginPlay)

(event Collision|EventActorBeginOverlap
  (params (OtherActor :type Actor%20Object%20Reference)))

(event EventTick
  (params (DeltaSeconds :type Float%20%28single-precision%29)))

(fn ConstructionScript)