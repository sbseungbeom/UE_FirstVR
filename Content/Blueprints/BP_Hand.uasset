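; BP_Hand is a VR hand actor that sets its mannequin mesh and motion controller source for left or right, and grabs objects.
; HandleGrab sphere-traces around the controller for a BP_GrabComponent, tries to grab it and stores it as held, while HandleRelease drops it.
; Both drive the grasp pose alpha in ABP_Hand.
; ResetHandMesh reattaches the mesh to the controller at the relative transform cached on BeginPlay.
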(event EventBeginPlay
  (Utilities|FlowControl|Sequence
    (:then_0
      (if (Variables|Default|GetbLeftHand)
        ;[1 1 1] 왼손
        (Variables|/Script/Engine.SkeletalMeshComponent|SetSkeletalMeshAsset (Variables|Default|GetHandMesh) "/Game/Sample/Characters/MannequinsXR/Meshes/SKM_MannyXR_left.SKM_MannyXR_left")
        (Transformation|SetRelativeRotation (Variables|Default|GetHandMesh) "180.000000,0.000000,-90.000000" false false)
        (Variables|/Script/HeadMountedDisplay.MotionControllerComponent|SetMotionSource (Variables|Default|GetMotionController) "Left")
        (else
          ;[1 1 1] 오른손
          (Variables|/Script/Engine.SkeletalMeshComponent|SetSkeletalMeshAsset (Variables|Default|GetHandMesh) "/Game/Sample/Characters/MannequinsXR/Meshes/SKM_MannyXR_right.SKM_MannyXR_right")
          (Transformation|SetRelativeRotation (Variables|Default|GetHandMesh) "0.000000,0.000000,90.000000" false false)
          (Variables|/Script/HeadMountedDisplay.MotionControllerComponent|SetMotionSource (Variables|Default|GetMotionController) "Right"))))
    (:then_1
      (Variables|Default|SetInitHandMeshRelativeTransform (Transformation|GetRelativeTransform (Variables|Default|GetHandMesh))))))

(event Collision|EventActorBeginOverlap
  (params (OtherActor :type Actor%20Object%20Reference)))

(fn ConstructionScript)

(fn HandleGrab
  (Utilities|FlowControl|Sequence
    (:then_0
      ;[1 1 1] GrabComponent가 있다면
      (bind _newparam (CallFunction|FindGrabComponentNearHand))
      (Utilities|IsValid _newparam
        (:Is%20Valid
          (bind _bsucess (Default|TryGrab _newparam self))
          (if _bsucess
            (bind _output_get (Variables|Default|SetHeldComponent _newparam))
            (Default|CallOnGrabbed _output_get)))))
    (:then_1
      (bind _asabp_hand (Utilities|Casting|CastToABP_Hand (Components|SkeletalMesh|GetAnimInstance (Variables|Default|GetHandMesh))))
      (Variables|/Game/Resources/Hand/ABP_Hand.ABP_Hand_C|SetPoseAlphaGrasp _asabp_hand 1.0))))

(fn HandleRelease
  (bind _heldcomponent (Variables|Default|GetHeldComponent))
  (Utilities|FlowControl|Sequence
    (:then_0
      (Utilities|IsValid _heldcomponent
        (:Is%20Valid
          (Default|CallOnDropped _heldcomponent)
          (Default|TryRelease _heldcomponent))))
    (:then_1
      (bind _asabp_hand (Utilities|Casting|CastToABP_Hand (Components|SkeletalMesh|GetAnimInstance (Variables|Default|GetHandMesh))))
      (Variables|/Game/Resources/Hand/ABP_Hand.ABP_Hand_C|SetPoseAlphaGrasp _asabp_hand 0.0))))

(fn FindGrabComponentNearHand
  (Utilities|FlowControl|Sequence
    (:then_0
      (bind _output_get (LocalVariables|SetLocalGripPosition (Transformation|GetWorldLocation (Variables|Default|GetMotionController))))
      (bind (_outhit _returnvalue) (Collision|SphereTraceForObjects _output_get _output_get (Variables|Default|GetGripRadius) (Utilities|Array|MakeArray "ObjectTypeQuery7") false 0 "ForDuration"))
      (if _returnvalue
        (Utilities|IsValid (Actor|GetComponentbyClass (.hitactor _outhit) "/Game/Blueprints/BP_GrabComponent.BP_GrabComponent_C")
          (:Is%20Valid
            (LocalVariables|SetLocalGrapComponent (Actor|GetComponentbyClass (.hitactor _outhit) "/Game/Blueprints/BP_GrabComponent.BP_GrabComponent_C"))))))
    (:then_1
      (return (LocalVariables|GetLocalGrapComponent)))))

(fn ResetHandMesh
  (Transformation|AttachComponentToComponent (Variables|Default|GetHandMesh) (Variables|Default|GetMotionController) "None" "KeepWorld" "KeepWorld" "KeepWorld" true)
  (Transformation|SetRelativeTransform (Variables|Default|GetHandMesh) (Variables|Default|GetInitHandMeshRelativeTransform) false true))