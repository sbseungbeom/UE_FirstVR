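; VR player pawn that handles smooth movement, snap turning and grabbing with two hands.
; On begin play it adds the VR input mapping, uses floor tracking, shifts VRRoot to a desired camera height after a delay, and attaches spawned BP_Hand actors to VRRoot.
; Enhanced Input moves along camera forward and forwards grab/release to each hand.
; SnapTurn rotates the actor, then offsets it to keep the camera's world position fixed.
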(event Input|EnhancedActionEvents|EnhancedInputActionIA_VR_Move
  (params (ActionValue :type Float%20%28double-precision%29) (ElapsedSeconds :type Float%20%28double-precision%29) (TriggeredSeconds :type Float%20%28double-precision%29) (InputAction :type Input%20Action%20Object%20Reference :default "/Game/Input/Actions/IA_VR_Move.IA_VR_Move"))
  (bind _camera (Variables|Default|GetCamera))
  (bind _returnvalue (Math|Vector|GetForwardVector _camera))
  (:Triggered
    (Pawn|Input|AddMovementInput (Math|Vector|MakeVector (.x _returnvalue) (.y _returnvalue) 0.0) ActionValue false)))

(event Input|EnhancedActionEvents|EnhancedInputActionIA_VR_Turn
  (params (ActionValue :type Float%20%28double-precision%29) (ElapsedSeconds :type Float%20%28double-precision%29) (TriggeredSeconds :type Float%20%28double-precision%29) (InputAction :type Input%20Action%20Object%20Reference :default "/Game/Input/Actions/IA_VR_Turn.IA_VR_Turn"))
  (:Started
    (CallFunction|SnapTurn (> ActionValue 0.0))))

(event Input|EnhancedActionEvents|EnhancedInputActionIA_VR_RightGrab
  (params (ActionValue :type Float%20%28double-precision%29) (ElapsedSeconds :type Float%20%28double-precision%29) (TriggeredSeconds :type Float%20%28double-precision%29) (InputAction :type Input%20Action%20Object%20Reference :default "/Game/Input/Actions/IA_VR_RightGrab.IA_VR_RightGrab"))
  (bind _righthand (Variables|Default|GetRightHand))
  (:Triggered
    (Default|HandleGrab _righthand))
  (:Completed
    (Default|HandleRelease _righthand)))

(event Input|EnhancedActionEvents|EnhancedInputActionIA_VR_LeftGrab
  (params (ActionValue :type Float%20%28double-precision%29) (ElapsedSeconds :type Float%20%28double-precision%29) (TriggeredSeconds :type Float%20%28double-precision%29) (InputAction :type Input%20Action%20Object%20Reference :default "/Game/Input/Actions/IA_VR_LeftGrab.IA_VR_LeftGrab"))
  (bind _lefthand (Variables|Default|GetLeftHand))
  (:Triggered
    (Default|HandleGrab _lefthand))
  (:Completed
    (Default|HandleRelease _lefthand)))

(event EventBeginPlay
  (Utilities|FlowControl|Sequence
    (:then_0
      (Input|AddMappingContext (PlayerController|LocalPlayerSubsystems|GetEnhancedInputLocalPlayerSubsystem (Game|GetPlayerController 0)) "/Game/Input/IMC_VR.IMC_VR" 0 "(bIgnoreAllPressedKeysUntilRelease=True,bForceImmediately=False)"))
    (:then_1
      (Class|HeadMountedDisplayFunctionLibrary|SetTrackingOrigin "Floor")
      (Utilities|FlowControl|Delay 1.0)
      (Transformation|AddRelativeLocation (Variables|Default|GetVRRoot) (Math|Vector|MakeVector 0.0 0.0 (- (Variables|Default|GetDesiredCameraHeight) (.z (Transformation|GetWorldLocation (Variables|Default|GetCamera))))) false false))
    (:then_2
      (bind _returnvalue (Game|SpawnActorfromClass "/Game/Blueprints/BP_Hand.BP_Hand_C" (Math|Transform|MakeTransform "0, 0, 0" "0, 0, 0" "1.000000,1.000000,1.000000") "AlwaysSpawn" self true 0))
      (bind _output_get (Variables|Default|SetLeftHand _returnvalue))
      (Transformation|AttachComponentToComponent _output_get (Variables|Default|GetVRRoot) "None" "SnapToTarget" "SnapToTarget" "KeepRelative" true))
    (:then_3
      (bind _returnvalue_2 (Game|SpawnActorfromClass "/Game/Blueprints/BP_Hand.BP_Hand_C" (Math|Transform|MakeTransform "0, 0, 0" "0, 0, 0" "1.000000,1.000000,1.000000") "AlwaysSpawn" self false 0))
      (bind _output_get_2 (Variables|Default|SetRightHand _returnvalue_2))
      (Transformation|AttachComponentToComponent _output_get_2 (Variables|Default|GetVRRoot) "None" "SnapToTarget" "SnapToTarget" "KeepRelative" true))))

(fn ConstructionScript)

(fn SnapTurn
  (params (bRightTurn :type Boolean))
  (bind _snapturndegrees (Variables|Default|GetSnapTurnDegrees))
  ;[1 1 1] PAWN 회전 시 위치 보정  Step 1.현재 카메라 위치 저장
  (LocalVariables|SetLocalCameraLocation (Transformation|GetWorldLocation (Variables|Default|GetCamera)))
  (Class|Actor|AddActorWorldRotation (Math|Rotator|MakeRotator 0.0 0.0 (Math|Float|SelectFloat (Math|Float|Absolute(Float) _snapturndegrees) _snapturndegrees bRightTurn)))
  ;[1 1 1] Step 2. 회전 후 camera위치와의 차이만큼 이동시킨다.
  (Transformation|AddActorWorldOffset (- (LocalVariables|GetLocalCameraLocation) (Transformation|GetWorldLocation (Variables|Default|GetCamera))) false true))