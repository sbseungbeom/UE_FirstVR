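; BP_Drawer is a VR drawer gimmick that slides along its forward axis while held by a motion controller.
; When its grab component fires OnGrabbed, it stores the controller and actor locations as reference points.
; Each Tick while grabbed, it projects the controller's displacement onto the actor's forward vector and teleports to that offset, with no sweep or travel limit.
; OnDropped clears the grabbed flag if the grabbing hand is still valid.
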(event OnGrabbed(BP_GrabComponent)
  (bind _bp_grabcomponent (Variables|Default|GetBP_GrabComponent))
  (bind _grabbinghand (Variables|/Game/Blueprints/BP_GrabComponent.BP_GrabComponent_C|GetGrabbingHand _bp_grabcomponent))
  (Utilities|IsValid _grabbinghand
    (:Is%20Valid
      (Variables|Default|SetMCGrabLocation (Transformation|GetWorldLocation (Variables|/Game/Blueprints/BP_Hand.BP_Hand_C|GetMotionController _grabbinghand)))
      (Variables|Default|SetActorGrabLocation (Transformation|GetActorLocation))
      (Variables|Default|SetGrabbed true))))

(event OnDropped(BP_GrabComponent)
  (Utilities|IsValid (Variables|/Game/Blueprints/BP_GrabComponent.BP_GrabComponent_C|GetGrabbingHand (Variables|Default|GetBP_GrabComponent))
    (:Is%20Valid
      (Variables|Default|SetGrabbed false))))

(event EventBeginPlay)

(event Collision|EventActorBeginOverlap
  (params (OtherActor :type Actor%20Object%20Reference)))

(event EventTick
  (params (DeltaSeconds :type Float%20%28single-precision%29))
  (bind _bp_grabcomponent (Variables|Default|GetBP_GrabComponent))
  (bind _grabbinghand (Variables|/Game/Blueprints/BP_GrabComponent.BP_GrabComponent_C|GetGrabbingHand _bp_grabcomponent))
  (if (Variables|Default|GetGrabbed)
    (Utilities|IsValid _grabbinghand
      (:Is%20Valid
        (Transformation|SetActorLocation (+ (Variables|Default|GetActorGrabLocation) (Math|Vector|ProjectVectorontoVector (- (Transformation|GetWorldLocation (Variables|/Game/Blueprints/BP_Hand.BP_Hand_C|GetMotionController _grabbinghand)) (Variables|Default|GetMCGrabLocation)) (Transformation|GetActorForwardVector))) false true)))))

(fn ConstructionScript)